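; Actor that scatters a random handful of obstacles, up/down arrows and gears (Engrenagem) inside its Box volume.
; The Construction Script rolls a count and a type per item, with obstacles weighted double and some rolls adding nothing.
; Helper functions add child actor components at random box points.
; Obstacles get random yaw and height scale, while arrows sit at a fixed height.
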(event `self.ReceiveBeginPlay`)

(event `self.ReceiveActorBeginOverlap`
  (params (OtherActor :type "Actor Object Reference")))

(event `self.ReceiveTick`
  (params (DeltaSeconds :type "Float (single-precision)")))

(fn `Add ArrowDown`
  (bind _box (`self.Box`))
  (`AddComponent|Child Actor Component_57` :`RelativeTransform` (`KismetMathLibrary.Conv_VectorToTransform` (`KismetMathLibrary.MakeVector` (.x (`KismetMathLibrary.RandomPointInBoundingBox` (`SceneComponent.RelativeLocation` _box) (`BoxComponent.BoxExtent` _box))) (.y (`KismetMathLibrary.RandomPointInBoundingBox` (`SceneComponent.RelativeLocation` _box) (`BoxComponent.BoxExtent` _box))) 50.0))))

(fn `Add ArrowUp`
  (bind _box (`self.Box`))
  (`AddComponent|Child Actor Component_58` :`RelativeTransform` (`KismetMathLibrary.Conv_VectorToTransform` (`KismetMathLibrary.MakeVector` (.x (`KismetMathLibrary.RandomPointInBoundingBox` (`SceneComponent.RelativeLocation` _box) (`BoxComponent.BoxExtent` _box))) (.y (`KismetMathLibrary.RandomPointInBoundingBox` (`SceneComponent.RelativeLocation` _box) (`BoxComponent.BoxExtent` _box))) 50.0))))

(fn `Add Engrenagem`
  (bind _box (`self.Box`))
  (`AddComponent|Child Actor Component_59` :`RelativeTransform` (`KismetMathLibrary.Conv_VectorToTransform` (`KismetMathLibrary.RandomPointInBoundingBox` (`SceneComponent.RelativeLocation` _box) (`BoxComponent.BoxExtent` _box)))))

(fn `Add Obstacle`
  (bind _box (`self.Box`))
  (`AddComponent|Child Actor Component_44` :`RelativeTransform` (`KismetMathLibrary.MakeTransform` (`KismetMathLibrary.RandomPointInBoundingBox` (`SceneComponent.RelativeLocation` _box) (`BoxComponent.BoxExtent` _box)) (`KismetMathLibrary.MakeRotator` (.roll (struct)) (.pitch (struct)) (+ (.yaw (struct)) (`KismetMathLibrary.RandomFloatInRange` -180.0 180.0))) (`KismetMathLibrary.MakeVector` (.x (1.0 1.0 1.0)) (.y (1.0 1.0 1.0)) (+ (.z (1.0 1.0 1.0)) (`KismetMathLibrary.RandomFloatInRange` -0.4 0.4))))))

(fn `UserConstructionScript`
  (for _ (range (+ (`KismetMathLibrary.RandomIntegerInRange` 0 4) 1))
    (switch `int` (`KismetMathLibrary.RandomIntegerInRange` 0 6)
      (:`1`
        (`self.Add Obstacle` :!label _label))
      (:`2`
        (goto _label))
      (:`3`
        (`self.Add ArrowUp`))
      (:`4`
        (`self.Add ArrowDown`))
      (:`5`
        (`self.Add Engrenagem`)))))