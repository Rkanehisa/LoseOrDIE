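; Espinhos_BP is a procedurally built spike field ("espinhos"), with its layout generated in the Construction Script.
; Nested loops over QuantidadeX and QuantidadeY add one static mesh component per cell, offset on a flat local grid by Distancia.
; Each cell is a separate component rather than an instance, and the event graph holds only disabled stubs, so no damage or overlap logic runs here.
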(event `self.ReceiveBeginPlay`)

(event `self.ReceiveActorBeginOverlap`
  (params (OtherActor :type "Actor Object Reference")))

(event `self.ReceiveTick`
  (params (DeltaSeconds :type "Float (single-precision)")))

(fn `UserConstructionScript`
  (for _index (range 1 (+ (`self.Quantidade x`) 1))
    (for _index_2 (range 1 (+ (`self.Quantidade y`) 1))
      (bind _returnvalue (`AddComponent|Static Mesh Component_274`))
      (`SceneComponent.K2_SetRelativeLocation` _returnvalue (`KismetMathLibrary.MakeVector` (* (- _index 1) (`self.Distancia`)) (* (- _index_2 1) (`self.Distancia`))) false false))))