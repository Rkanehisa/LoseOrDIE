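; BP_Track is a floor tile for a runner game with a self-extending track.
; When the RunCharacter enters EndTrigger, it asks RunGameMode once to add a tile, then destroys itself two seconds later.
; Another BP_Track overlapping that trigger is stored as NextTrack, and GetAttachTransform exposes the AttachPoint's world transform.
; Hits on either side wall call TakeHit on the character.
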(event `self.ReceiveBeginPlay`)

(event `self.ReceiveActorBeginOverlap`
  (params (OtherActor :type "Actor Object Reference")))

(event `self.ReceiveTick`
  (params (DeltaSeconds :type "Float (single-precision)")))

(event `self.EndTrigger.OnComponentBeginOverlap`
  (params (OtherActor :type "Actor Object Reference") (OtherComp :type "PrimitiveComponent Object Reference") (OtherBodyIndex :type Integer) (bFromSweep :type Boolean) (SweepResult :type "HitResult Structure (by ref)"))
  (cast `/Game/ThirdPersonBP/Blueprints/RunCharacter` OtherActor
    (:`then`
      (bind _asrun_game_mode (cast `/Game/ThirdPersonBP/Blueprints/RunGameMode` (`GameplayStatics.GetGameMode`)))
      (`/Engine/EditorBlueprintResources/StandardMacros.DoOnce` false
        (:`Completed`
          (`/Game/ThirdPersonBP/Blueprints/RunGameMode.AddFloorTile` _asrun_game_mode)
          (`KismetSystemLibrary.Delay` 2.0)
          (`self.K2_DestroyActor`))))
    (:`CastFailed`
      (bind _asbp_track (cast `/Game/Track/BP_Track` OtherActor))
      (set `self.NextTrack` _asbp_track))))

(event `self.WallR.OnComponentHit`
  (params (OtherActor :type "Actor Object Reference") (OtherComp :type "PrimitiveComponent Object Reference") (NormalImpulse :type "Vector Structure") (Hit :type "HitResult Structure (by ref)"))
  (bind _asrun_character (cast `/Game/ThirdPersonBP/Blueprints/RunCharacter` OtherActor))
  (`/Game/ThirdPersonBP/Blueprints/RunCharacter.TakeHit` _asrun_character))

(event `self.WallL.OnComponentHit`
  (params (OtherActor :type "Actor Object Reference") (OtherComp :type "PrimitiveComponent Object Reference") (NormalImpulse :type "Vector Structure") (Hit :type "HitResult Structure (by ref)"))
  (bind _asrun_character (cast `/Game/ThirdPersonBP/Blueprints/RunCharacter` OtherActor))
  (`/Game/ThirdPersonBP/Blueprints/RunCharacter.TakeHit` _asrun_character))

(fn `GetAttachTransform`
  (returns (AttachTransform :type "Transform Structure"))
  (return (`SceneComponent.K2_GetComponentToWorld` (`self.AttachPoint`))))

(fn `UserConstructionScript`)