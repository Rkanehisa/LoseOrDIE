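; Track segment for a runner game that scatters random items across itself and has side walls that damage the player.
; The construction script makes a random number of picks among arrow-down, gear, arrow-up and pedra (rock) spawners, so the layout rerolls whenever construction runs.
; Each spawner adds a child actor component at a random XY inside BlockerArea with a fixed height.
; Hits on WallL or WallR call TakeHit on the RunCharacter.
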(event `self.ReceiveBeginPlay`)

(event `self.ReceiveActorBeginOverlap`
  (params (OtherActor :type "Actor Object Reference")))

(event `self.ReceiveTick`
  (params (DeltaSeconds :type "Float (single-precision)")))

(event `self.WallR.OnComponentHit`
  (params (OtherActor :type "Actor Object Reference") (OtherComp :type "PrimitiveComponent Object Reference") (NormalImpulse :type "Vector Structure") (Hit :type "HitResult Structure (by ref)"))
  (bind _asrun_character (cast `/Game/ThirdPersonBP/Blueprints/RunCharacter` OtherActor))
  (`/Game/ThirdPersonBP/Blueprints/RunCharacter.TakeHit` _asrun_character))

(event `self.WallL.OnComponentHit`
  (params (OtherActor :type "Actor Object Reference") (OtherComp :type "PrimitiveComponent Object Reference") (NormalImpulse :type "Vector Structure") (Hit :type "HitResult Structure (by ref)"))
  (bind _asrun_character (cast `/Game/ThirdPersonBP/Blueprints/RunCharacter` OtherActor))
  (`/Game/ThirdPersonBP/Blueprints/RunCharacter.TakeHit` _asrun_character))

(fn `SpawnArrowDown`
  (bind _blockerarea (`self.BlockerArea`))
  (`AddComponent|Child Actor Component_4` :`RelativeTransform` (`KismetMathLibrary.Conv_VectorToTransform` (`KismetMathLibrary.MakeVector` (.x (`KismetMathLibrary.RandomPointInBoundingBox` (`SceneComponent.RelativeLocation` _blockerarea) (`BoxComponent.BoxExtent` _blockerarea))) (.y (`KismetMathLibrary.RandomPointInBoundingBox` (`SceneComponent.RelativeLocation` _blockerarea) (`BoxComponent.BoxExtent` _blockerarea))) 50.0))))

(fn `SpawnArrowUP`
  (bind _blockerarea (`self.BlockerArea`))
  (`AddComponent|Child Actor Component_115` :`RelativeTransform` (`KismetMathLibrary.Conv_VectorToTransform` (`KismetMathLibrary.MakeVector` (.x (`KismetMathLibrary.RandomPointInBoundingBox` (`SceneComponent.RelativeLocation` _blockerarea) (`BoxComponent.BoxExtent` _blockerarea))) (.y (`KismetMathLibrary.RandomPointInBoundingBox` (`SceneComponent.RelativeLocation` _blockerarea) (`BoxComponent.BoxExtent` _blockerarea))) 50.0))))

(fn `SpawnGear`
  (bind _blockerarea (`self.BlockerArea`))
  (`AddComponent|Child Actor Component_8` :`RelativeTransform` (`KismetMathLibrary.Conv_VectorToTransform` (`KismetMathLibrary.MakeVector` (.x (`KismetMathLibrary.RandomPointInBoundingBox` (`SceneComponent.RelativeLocation` _blockerarea) (`BoxComponent.BoxExtent` _blockerarea))) (.y (`KismetMathLibrary.RandomPointInBoundingBox` (`SceneComponent.RelativeLocation` _blockerarea) (`BoxComponent.BoxExtent` _blockerarea))) 50.0))))

(fn `SpawnPedra`
  (bind _blockerarea (`self.BlockerArea`))
  (`AddComponent|Child Actor Component_46` :`RelativeTransform` (`KismetMathLibrary.Conv_VectorToTransform` (`KismetMathLibrary.MakeVector` (.x (`KismetMathLibrary.RandomPointInBoundingBox` (`SceneComponent.RelativeLocation` _blockerarea) (`BoxComponent.BoxExtent` _blockerarea))) (.y (`KismetMathLibrary.RandomPointInBoundingBox` (`SceneComponent.RelativeLocation` _blockerarea) (`BoxComponent.BoxExtent` _blockerarea))) 0.0))))

(fn `UserConstructionScript`
  (`parent.UserConstructionScript`)
  (for _ (range (+ (`KismetMathLibrary.RandomIntegerInRange` 0 3) 1))
    (switch `int` (`KismetMathLibrary.RandomIntegerInRange` 0 3)
      (:`0`
        (`self.SpawnArrowDown`))
      (:`1`
        (`self.SpawnGear`))
      (:`2`
        (`self.SpawnArrowUP`))
      (:`3`
        (`self.SpawnPedra`)))))