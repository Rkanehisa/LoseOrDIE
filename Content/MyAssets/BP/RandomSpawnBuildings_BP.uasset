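; Construction-script Blueprint that scatters randomized building child actors across positions marked by billboard components.
; AddToArray collects the billboards' relative transforms, plus two unwired entries, into PositionArray.
; SpawnRandomBuildings loops over it, randomly skipping some slots and adding child actors at the rest, with either random height or random yaw and non-uniform scale.
; The layout re-rolls whenever construction reruns, as no seeded stream is used.
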(event `self.ReceiveBeginPlay`)

(event `self.ReceiveActorBeginOverlap`
  (params (OtherActor :type "Actor Object Reference")))

(event `self.ReceiveTick`
  (params (DeltaSeconds :type "Float (single-precision)")))

(fn `AddToArray`
  (set `self.PositionArray` (`|MakeArray` (`SceneComponent.GetRelativeTransform` (`self.Billboard5`)) (`SceneComponent.GetRelativeTransform` (`self.Billboard4`)) (`SceneComponent.GetRelativeTransform` (`self.Billboard3`)) (`SceneComponent.GetRelativeTransform` (`self.Billboard2`)) (`SceneComponent.GetRelativeTransform` (`self.Billboard1`)) (`SceneComponent.GetRelativeTransform` (`self.Billboard`)) (struct) (struct))))

(fn `SpawnRandomBuildings`
  (bind _returnvalue (`KismetMathLibrary.RandomIntegerInRange` 0 3))
  (bind _returnvalue_2 (`KismetMathLibrary.RandomFloatInRange` 0.8 2.0))
  (for _array_element (`self.PositionArray`)
    (if (== _returnvalue 0)
      _
      (elif (== _returnvalue 1)
        (`AddComponent|Child Actor Component_33` :`RelativeTransform` (`KismetMathLibrary.MakeTransform` (`KismetMathLibrary.MakeVector` (.x (.location _array_element)) (.y (.location _array_element)) (`KismetMathLibrary.RandomFloatInRange` 0.0 200.0))))
        (else
          (`AddComponent|Child Actor Component_2` :`RelativeTransform` (`KismetMathLibrary.MakeTransform` (.location _array_element) (`KismetMathLibrary.MakeRotator` 0.0 0.0 (`KismetMathLibrary.RandomFloatInRange` 0.0 359.0)) (`KismetMathLibrary.MakeVector` _returnvalue_2 _returnvalue_2 (`KismetMathLibrary.RandomFloatInRange` 0.8 1.7)))))))))

(fn `UserConstructionScript`
  (`self.AddToArray`)
  (`self.SpawnRandomBuildings`))