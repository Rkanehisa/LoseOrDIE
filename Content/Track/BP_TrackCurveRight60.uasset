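; Curved track piece for a runner game, representing a 60-degree right turn.
; Its CurvaCollision overlap sets the RunCharacter's Angulo to 60 and enables CanTurn through a DoOnce that resets after a short delay.
; If a BP_Track overlaps that trigger instead, it is stored as NextTrack.
; Hits on any of the curve or wall components call TakeHit on the runner.
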(event `self.ReceiveBeginPlay`)

(event `self.ReceiveActorBeginOverlap`
  (params (OtherActor :type "Actor Object Reference")))

(event `self.ReceiveTick`
  (params (DeltaSeconds :type "Float (single-precision)")))

(event `self.CurvaCollision.OnComponentBeginOverlap`
  (params (OtherActor :type "Actor Object Reference") (OtherComp :type "PrimitiveComponent Object Reference") (OtherBodyIndex :type Integer) (bFromSweep :type Boolean) (SweepResult :type "HitResult Structure (by ref)"))
  (bind _asrun_character (cast `/Game/ThirdPersonBP/Blueprints/RunCharacter` OtherActor)
    (:`then`
      (set `/Game/ThirdPersonBP/Blueprints/RunCharacter.Angulo` 60.0 _asrun_character)
      (`/Engine/EditorBlueprintResources/StandardMacros.DoOnce` false :!label _label
        (:`Completed`
          (set `/Game/ThirdPersonBP/Blueprints/RunCharacter.CanTurn` true _asrun_character)
          (`KismetSystemLibrary.Delay` 0.5)
          (goto _label :!via `Reset`))))
    (:`CastFailed`
      (bind _asbp_track (cast `/Game/Track/BP_Track` OtherActor))
      (set `self.NextTrack` _asbp_track))))

(event `self.CurveR.OnComponentHit`
  (params (OtherActor :type "Actor Object Reference") (OtherComp :type "PrimitiveComponent Object Reference") (NormalImpulse :type "Vector Structure") (Hit :type "HitResult Structure (by ref)"))
  (bind _asrun_character (cast `/Game/ThirdPersonBP/Blueprints/RunCharacter` OtherActor))
  (`/Game/ThirdPersonBP/Blueprints/RunCharacter.TakeHit` _asrun_character))

(event `self.WallR.OnComponentHit`
  (params (OtherActor :type "Actor Object Reference") (OtherComp :type "PrimitiveComponent Object Reference") (NormalImpulse :type "Vector Structure") (Hit :type "HitResult Structure (by ref)"))
  (bind _asrun_character (cast `/Game/ThirdPersonBP/Blueprints/RunCharacter` OtherActor))
  (`/Game/ThirdPersonBP/Blueprints/RunCharacter.TakeHit` _asrun_character))

(event `self.WallL.OnComponentHit`
  (params (OtherActor :type "Actor Object Reference") (OtherComp :type "PrimitiveComponent Object Reference") (NormalImpulse :type "Vector Structure") (Hit :type "HitResult Structure (by ref)"))
  (bind _asrun_character (cast `/Game/ThirdPersonBP/Blueprints/RunCharacter` OtherActor))
  (`/Game/ThirdPersonBP/Blueprints/RunCharacter.TakeHit` _asrun_character))

(event `self.WallEndR.OnComponentHit`
  (params (OtherActor :type "Actor Object Reference") (OtherComp :type "PrimitiveComponent Object Reference") (NormalImpulse :type "Vector Structure") (Hit :type "HitResult Structure (by ref)"))
  (bind _asrun_character (cast `/Game/ThirdPersonBP/Blueprints/RunCharacter` OtherActor))
  (`/Game/ThirdPersonBP/Blueprints/RunCharacter.TakeHit` _asrun_character))

(event `self.WallEndL.OnComponentHit`
  (params (OtherActor :type "Actor Object Reference") (OtherComp :type "PrimitiveComponent Object Reference") (NormalImpulse :type "Vector Structure") (Hit :type "HitResult Structure (by ref)"))
  (bind _asrun_character (cast `/Game/ThirdPersonBP/Blueprints/RunCharacter` OtherActor))
  (`/Game/ThirdPersonBP/Blueprints/RunCharacter.TakeHit` _asrun_character))

(event `self.CurveL.OnComponentHit`
  (params (OtherActor :type "Actor Object Reference") (OtherComp :type "PrimitiveComponent Object Reference") (NormalImpulse :type "Vector Structure") (Hit :type "HitResult Structure (by ref)"))
  (bind _asrun_character (cast `/Game/ThirdPersonBP/Blueprints/RunCharacter` OtherActor))
  (`/Game/ThirdPersonBP/Blueprints/RunCharacter.TakeHit` _asrun_character))

(fn `UserConstructionScript`
  (`parent.UserConstructionScript`))